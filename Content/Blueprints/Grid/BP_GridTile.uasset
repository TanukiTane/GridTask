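; BP_GridTile is a single grid tile actor that shows its ground type and its hovered, selected and path states.
; Cursor hover and clicks on the Cube update the tile and notify BPGrid, which holds the tile data looked up by GridIndex.
; SetTileColor layers ground color, hover brightening and path override into material parameters, with selection as a separate scalar.
; BeginPlay waits briefly before coloring and passing the grid and index to its WBP_GridTile widget.
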(event OnBeginCursorOver(Cube)
  (params (TouchedComponent :type Primitive%20Component%20Object%20Reference))
  (CallFunction|EventStartOverTile)
  (Default|EventNewTileOvered (Variables|Grid|GetBP_Grid) self))

(event OnClicked(Cube)
  (params (TouchedComponent :type Primitive%20Component%20Object%20Reference) (ButtonPressed :type Key%20Structure :default "None"))
  (CallFunction|EventSelectTile)
  (Default|EventNewTileSelected (Variables|Grid|GetBP_Grid) self))

(event Custom|Event_SelectTile
  (Variables|Grid|SetbisSelected true)
  (Grid|SetTileColor))

(event Custom|Event_DeselectTile
  (Variables|Grid|SetbisSelected false)
  (Grid|SetTileColor))

(event Custom|Event_EndOverTile
  (Variables|Grid|SetbisOvered false)
  (Grid|SetTileColor))

(event Custom|Event_StartOverTile
  (Variables|Grid|SetbisOvered true)
  (Grid|SetTileColor))

(event Custom|Event_IsInPath
  (params (bIsInPath :type Boolean))
  (Variables|Default|SetbIsInPath bIsInPath)
  (Grid|SetTileColor))

(event EventBeginPlay
  (Utilities|FlowControl|Delay 0.5)
  (Grid|SetTileColor)
  (CallFunction|SetWidgetVar))

(event Collision|EventActorBeginOverlap
  (params (OtherActor :type Actor%20Object%20Reference)))

(event EventTick
  (params (DeltaSeconds :type Float%20%28single-precision%29)))

(fn ConstructionScript)

(fn SetTileColor
  (Utilities|FlowControl|Sequence
    (:then_0
      ;[1 1 1] Set Color On Enum
      (switch Utilities|FlowControl|Switch|SwitchonE_GroundType (.groundtype (Grid|GetTileData))
        (:NewEnumerator0
          (LocalVariables|SetTileColor "(R=0.000000,G=1.000000,B=0.182862,A=1.000000)"))
        (:NewEnumerator1
          (LocalVariables|SetTileColor "(R=0.858335,G=1.000000,B=0.003805,A=1.000000)"))
        (:NewEnumerator2
          (LocalVariables|SetTileColor "(R=1.000000,G=0.510500,B=0.000000,A=1.000000)"))
        (:NewEnumerator3
          (LocalVariables|SetTileColor "(R=1.000000,G=0.000000,B=0.000000,A=1.000000)"))
        (:NewEnumerator4
          (LocalVariables|SetTileColor "(R=0.130208,G=0.130208,B=0.130208,A=1.000000)"))))
    (:then_1
      ;[1 1 1] For Selected
      (if (Variables|Grid|GetbisSelected)
        (Rendering|Material|SetScalarParameterValueonMaterials (Variables|Default|GetCube) "bisSelected" 2e+01)
        (else
          (Rendering|Material|SetScalarParameterValueonMaterials (Variables|Default|GetCube) "bisSelected" 0.0))))
    (:then_2
      ;[1 1 1] For Overed
      (if (Variables|Grid|GetbisOvered)
        (LocalVariables|SetTileColor (Math|Conversions|ToLinearColor(Vector) (* (Math|Conversions|ToVector(LinearColor) (LocalVariables|GetTileColor)) 3.0)))))
    (:then_3
      ;[1 1 1] For Path
      (if (Variables|Default|GetbIsInPath)
        (LocalVariables|SetTileColor "(R=0.066727,G=0.065923,B=0.359375,A=1.000000)")))
    (:then_4
      ;[1 1 1] SetColor
      (Rendering|Material|SetVectorParameterValueonMaterials (Variables|Default|GetCube) "TileColor" (Math|Conversions|ToVector(LinearColor) (LocalVariables|GetTileColor))))))

(fn GetTileData
  (return (.Value (Utilities|Map|Find (Variables|/Game/Blueprints/Grid/BP_Grid.BP_Grid_C|GetStr_Tiles (Variables|Grid|GetBP_Grid)) (Variables|Grid|GetGridIndex)))))

(fn SetTileSize
  (bind _bp_grid (Variables|Grid|GetBP_Grid))
  (bind _cube (Variables|Default|GetCube))
  (bind _returnvalue (Transformation|GetWorldScale _cube))
  (bind _tilesize (Variables|/Game/Blueprints/Grid/BP_Grid.BP_Grid_C|GetTileSize _bp_grid))
  (bind _returnvalue_2 (/ _tilesize 5e+01))
  (bind _returnvalue_3 (/ _returnvalue _returnvalue_2))
  (Transformation|SetWorldScale3D _cube (Math|Vector|MakeVector (.x _returnvalue_3) (.y _returnvalue_3) 1.0)))

(fn SetWidgetVar
  (bind _widget (Variables|Default|GetWidget))
  (bind _returnvalue (UserInterface|GetUserWidgetObject _widget))
  (bind _aswbp_grid_tile (Utilities|Casting|CastToWBP_GridTile _returnvalue))
  (Variables|/Game/Blueprints/Grid/WBP_GridTile.WBP_GridTile_C|SetGrid _aswbp_grid_tile (Variables|Grid|GetBP_Grid))
  (Variables|/Game/Blueprints/Grid/WBP_GridTile.WBP_GridTile_C|SetgridIndex _aswbp_grid_tile (Variables|Grid|GetGridIndex)))